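; Player controller that creates the primary HUD and handles movement, look, jump, melee attack and Gameplay Ability System input.
; Five slot inputs fetch the ability class stored in the matching UI slot and activate it on the controlled BP_CharacterBase.
; Activation also sets the character's Targeting flag for target-type abilities and calls TargetCancel, while a cancel input aborts all abilities.
; AddAbilitytoUI forwards new ability info into the HUD slots.
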(event `self.ReceiveBeginPlay`
  (bind _returnvalue (`|CreateWidget` "/Game/UI/WBP_PrimaryUI.WBP_PrimaryUI_C"))
  (bind _output_get (set `self.PrimaryUI` _returnvalue))
  (`UserWidget.AddToViewport` _output_get 0))

(event `InputAxis|MoveForward`
  (params (AxisValue :type "Float (single-precision)"))
  ;[1 1 1] Player Control
  (`Pawn.AddMovementInput` (`self.K2_GetPawn`) (`KismetMathLibrary.GetForwardVector` (`PlayerCameraManager.GetCameraRotation` (`self.PlayerCameraManager`))) AxisValue false))

(event `self.AddAbilityToUI`
  (params (AbilityInfo :type "GameplayAbilityInfo Structure"))
  ;[1 1 1] Add Abilities To UI
  (`/Game/UI/WBP_PrimaryUI.AddAbilityToSlots` (`self.PrimaryUI`) AbilityInfo))

(event `InputAxis|MoveRight`
  (params (AxisValue :type "Float (single-precision)"))
  ;[1 1 1] Player Control
  (`Pawn.AddMovementInput` (`self.K2_GetPawn`) (`KismetMathLibrary.GetRightVector` (`PlayerCameraManager.GetCameraRotation` (`self.PlayerCameraManager`))) AxisValue false))

(event `InputAction|SlotOneAbility`
  (params (Key :type "Key Structure"))
  ;[1 1 1] Ability Input
  (:`Pressed`
    (`self.TryActivateAbilityInUISlot` 0)))

(event `InputAction|Jump`
  (params (Key :type "Key Structure"))
  (bind _returnvalue (`GameplayStatics.GetPlayerCharacter` 0))
  ;[1 1 1] Player Control
  (:`Pressed`
    (`Character.Jump` _returnvalue))
  (:`Released`
    (`Character.StopJumping` _returnvalue)))

(event `InputAction|SlotTwoAbility`
  (params (Key :type "Key Structure"))
  ;[1 1 1] Ability Input
  (:`Pressed`
    (`self.TryActivateAbilityInUISlot` 1)))

(event `InputAction|SlotThreeAbility`
  (params (Key :type "Key Structure"))
  ;[1 1 1] Ability Input
  (:`Pressed`
    (`self.TryActivateAbilityInUISlot` 2)))

(event `InputAction|SlotFourAbility`
  (params (Key :type "Key Structure"))
  ;[1 1 1] Ability Input
  (:`Pressed`
    (`self.TryActivateAbilityInUISlot` 3)))

(event `InputAxis|LookUp`
  (params (AxisValue :type "Float (single-precision)"))
  ;[1 1 1] Player Control
  (`self.AddPitchInput` AxisValue))

(event `InputAxis|Turn`
  (params (AxisValue :type "Float (single-precision)"))
  ;[1 1 1] Player Control
  (`self.AddYawInput` AxisValue))

(event `InputAction|SlotFiveAbility`
  (params (Key :type "Key Structure"))
  ;[1 1 1] Ability Input
  (:`Pressed`
    (`self.TryActivateAbilityInUISlot` 4)))

(event `InputAction|CancelAbility`
  (params (Key :type "Key Structure"))
  ;[1 1 1] Ability Input
  (:`Pressed`
    (bind _asbp_character_base (cast `/Game/Blueprints/Characters/BP_CharacterBase` (`self.K2_GetPawn`)))
    (`CharacterBase.CancelAllAbilities` _asbp_character_base)
    (`AbilitySystemComponent.TargetCancel` (`CharacterBase.AbilitySystemComp` _asbp_character_base))))

(event `InputAction|PrimaryAttack`
  (params (Key :type "Key Structure"))
  ;[1 1 1] Primary Attack
  (:`Pressed`
    (bind _asbp_character_base (cast `/Game/Blueprints/Characters/BP_CharacterBase` (`self.K2_GetPawn`)))
    (`/Game/Blueprints/Characters/BP_CharacterBase.MeleeAttack` _asbp_character_base)))

(fn `TryActivateAbilityInUISlot`
  (params (SlotNumber :type Integer))
  (bind (_abilityclass _isvalid) (`/Game/UI/WBP_PrimaryUI.GetSlotAbilityClass` (`self.PrimaryUI`) SlotNumber))
  (if _isvalid
    (bind _asbp_character_base (cast `/Game/Blueprints/Characters/BP_CharacterBase` (`self.K2_GetPawn`)))
    (`AbilitySystemComponent.TryActivateAbilityByClass` (`AbilitySystemBlueprintLibrary.GetAbilitySystemComponent` _asbp_character_base) _abilityclass true)
    (castclass `/Game/Blueprints/Characters/GameplayAbilities/BP_GameplayAbilityTarget` _abilityclass
      (:`then`
        (set `/Game/Blueprints/Characters/BP_CharacterBase.Targeting` true _asbp_character_base))
      (:`CastFailed`
        (set `/Game/Blueprints/Characters/BP_CharacterBase.Targeting` false _asbp_character_base)))
    (`AbilitySystemComponent.TargetCancel` (`AbilitySystemBlueprintLibrary.GetAbilitySystemComponent` _asbp_character_base))))

(fn `UserConstructionScript`)