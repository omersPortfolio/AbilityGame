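; GA_Lazer is a gameplay ability that casts a damaging laser beam from the character while its cost remains available.
; On activation it commits, plays the casting montage, attaches a spawned BP_Lazer to the mesh socket and enables camera-controlled rotation.
; Damage gameplay events apply GE_Lazer_Damage and push targets with a stun, unless key 3 cancels or cost runs out.
; Ending removes the draining cost effect, destroys the beam and restores rotation.
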(event `self.K2_ActivateAbility`
  (`self.K2_CommitAbility`)
  (`self.ImplementUICooldown`)
  (`AbilityTask_PlayMontageAndWait.CreatePlayMontageAndWaitProxy` "None" "/Game/Blueprints/Characters/Animation/AM_Lazer_Casting.AM_Lazer_Casting"
    (:`then`
      (`KismetSystemLibrary.Delay` 0.4)
      (bind _character (`self.GetPlayerAndController`))
      (bind (_asynctaskproxy _spawnedactor) (`AbilityTask_SpawnActor.SpawnActor` (struct) "/Game/Blueprints/Characters/GameplayAbilities/Lazer/BP_Lazer.BP_Lazer_C" _character)
        (:`then`
          (bind _output_get (set `self.LazerActor` _spawnedactor))
          (`Actor.K2_AttachToComponent` _output_get (`Character.Mesh` _character) "Lazer" "SnapToTarget" "SnapToTarget" "KeepRelative" true)
          (`/Game/Blueprints/Characters/BP_CharacterBase.ToggleCameraControlRotation` _character true)
          (bind (_asynctaskproxy_2 _payload) (`AbilityTask_WaitGameplayEvent.WaitGameplayEvent` (struct :`TagName` "skill.lazer.dealDamage") null)
            (:`EventReceived`
              (bind (_character_2 _playercontroller) (`self.GetPlayerAndController`))
              (if (`PlayerController.IsInputKeyDown` _playercontroller "Three")
                (`self.K2_CancelAbility`)
                (else
                  (bind _can (`self.IsCostStillAvailable`))
                  (if _can
                    (bind (_eventtag _instigator _target _optionalobject _optionalobject2 _contexthandle _instigatortags _targettags _eventmagnitude _targetdata) (break `GameplayEventData` _payload))
                    (`self.BP_ApplyGameplayEffectToTarget` _targetdata "/Game/Blueprints/Characters/GameplayAbilities/Lazer/GE_Lazer_Damage.GE_Lazer_Damage_C")
                    (for _array_element (`AbilitySystemBlueprintLibrary.GetActorsFromTargetData` _targetdata)
                      (bind _asbp_character_base (cast `/Game/Blueprints/Characters/BP_CharacterBase` _array_element))
                      (`/Game/Blueprints/Characters/BP_CharacterBase.PushCharacter` _asbp_character_base (`KismetMathLibrary.Normal` (- (`Actor.K2_GetActorLocation` _asbp_character_base) (`SceneComponent.K2_GetComponentLocation` (`/Game/Blueprints/Characters/GameplayAbilities/Lazer/BP_Lazer.LazerEndDetector` (cast `/Game/Blueprints/Characters/GameplayAbilities/Lazer/BP_Lazer` (`self.LazerActor`) :!pure true))))) 500.0 0.3))
                    (else
                      (`self.K2_EndAbility`))))))))))))

(event `self.K2_OnEndAbility`
  (params (bWasCancelled :type Boolean))
  (bind _lazeractor (`self.LazerActor`))
  (`self.BP_RemoveGameplayEffectFromOwnerWithAssetTags` (struct :`GameplayTags` (struct :`(TagName` "skill.lazer.drainingCost"))))
  (`/Engine/EditorBlueprintResources/StandardMacros.IsValid` _lazeractor
    (:`Is Valid`
      (`Actor.K2_DestroyActor` _lazeractor)
      (bind _character (`self.GetPlayerAndController`))
      (`/Game/Blueprints/Characters/BP_CharacterBase.ToggleCameraControlRotation` _character false))))