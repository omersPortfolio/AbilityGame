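; Base Gameplay Ability Blueprint that supplies shared helper functions for character abilities, with no activation logic of its own.
; It resolves the owning BP_CharacterBase and its player controller, then uses the controller's PrimaryUI to start cooldowns on slots matching the ability's class.
; A cost check negates the ability info's cost and compares it against the character's current Health, Mana or Strength attribute, selected by cost type.
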(fn `GetPlayerAndController`
  (returns (Character :type "/Game/Blueprints/Characters/BP_CharacterBase Object Reference") (PlayerController :type "/Game/Blueprints/BP_PlayerController Object Reference"))
  (bind _asbp_character_base (cast `/Game/Blueprints/Characters/BP_CharacterBase` (`self.GetOwningActorFromActorInfo`)))
  (bind _asbp_player_controller (cast `/Game/Blueprints/BP_PlayerController` (`Pawn.GetController` _asbp_character_base))
    (:`then`
      _)
    (:`CastFailed`
      _))
  (return _asbp_character_base _asbp_player_controller))

(fn `ImplementUICooldown`
  (bind (_character _playercontroller) (`self.GetPlayerAndController`))
  (`/Engine/EditorBlueprintResources/StandardMacros.IsValid` _playercontroller
    (:`Is Valid`
      (for _array_element (`/Game/UI/WBP_PrimaryUI.AbilitySlots` (`/Game/Blueprints/BP_PlayerController.PrimaryUI` _playercontroller))
        (bind _returnvalue (`self.GetAbilityInfo`))
        (bind (_abilityinfo_cooldownduration _abilityinfo_cost _abilityinfo_costtype _abilityinfo_uimat _abilityinfo_abilityclass) (break `GameplayAbilityInfo` (`/Game/UI/WBP_AbilitySlot.AbilityInfo` _array_element)))
        (if (== _abilityinfo_abilityclass (`.AbilityClass` (break `GameplayAbilityInfo` _returnvalue)))
          (`/Game/UI/WBP_AbilitySlot.StartCooldown` _array_element))))))

(fn `IsCostStillAvailable`
  (returns (Can :type Boolean))
  (locals (Cost :type "Float (double-precision)"))
  (bind _returnvalue (`self.GetAbilityInfo`))
  (set `local.Cost` (* (`.Cost` (break `GameplayAbilityInfo` _returnvalue)) -1.0))
  (switch `EAbilityCostType` (`.CostType` (break `GameplayAbilityInfo` _returnvalue))
    (:`Health`
      (bind _character (`self.GetPlayerAndController`))
      (bind (_health_basevalue _health_currentvalue) (break `GameplayAttributeData` (`AttributeSetBase.Health` (`CharacterBase.AttributeSetBaseComp` _character))))
      (return (>= _health_currentvalue (`local.Cost`))))
    (:`Mana`
      (bind _character_2 (`self.GetPlayerAndController`))
      (bind (_mana_basevalue _mana_currentvalue) (break `GameplayAttributeData` (`AttributeSetBase.Mana` (`CharacterBase.AttributeSetBaseComp` _character_2))))
      (return (>= _mana_currentvalue (`local.Cost`))))
    (:`Strength`
      (bind _character_3 (`self.GetPlayerAndController`))
      (bind (_strength_basevalue _strength_currentvalue) (break `GameplayAttributeData` (`AttributeSetBase.Strength` (`CharacterBase.AttributeSetBaseComp` _character_3))))
      (return (>= _strength_currentvalue (`local.Cost`))))))