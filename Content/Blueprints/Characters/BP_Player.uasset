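; BP_Player is the player character Blueprint that keeps the HUD's health and mana glass balls in sync with the character's stats.
; OnHealthChanged and OnManaChanged each cast the controller to BP_PlayerController, then set the matching ball on its PrimaryUI to current divided by maximum.
; Either update silently stops if that cast fails, and the construction script only calls its parent.
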(event `self.BP_OnHealthChanged`
  (params (Health :type "Float (single-precision)") (MaxHealth :type "Float (single-precision)"))
  (bind _asbp_player_controller (cast `/Game/Blueprints/BP_PlayerController` (`self.GetController`)))
  (`/Game/UI/WBP_GlassBall.SetPercentage` (`/Game/UI/WBP_PrimaryUI.HealthGlassBall` (`/Game/Blueprints/BP_PlayerController.PrimaryUI` _asbp_player_controller)) (/ Health MaxHealth)))

(event `self.BP_OnManaChanged`
  (params (Mana :type "Float (single-precision)") (MaxMana :type "Float (single-precision)"))
  (bind _asbp_player_controller (cast `/Game/Blueprints/BP_PlayerController` (`self.GetController`)))
  (`/Game/UI/WBP_GlassBall.SetPercentage` (`/Game/UI/WBP_PrimaryUI.ManaGlassBall` (`/Game/Blueprints/BP_PlayerController.PrimaryUI` _asbp_player_controller)) (/ Mana MaxMana)))

(fn `UserConstructionScript`
  (`parent.UserConstructionScript`))