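; Base character Blueprint using the Gameplay Ability System for melee and dash combat, granting initial abilities on BeginPlay.
; Melee input activates GA_Melee, or confirms the target while targeting.
; Sword and capsule overlaps with hostile characters send damage gameplay events to itself, with an exclude list preventing repeat dash hits.
; Also handles montage-timed death, zero-friction knockback with optional stun, and toggles for rotation mode and pawn collision.
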(event `MeleeAttack`
  ;[1 1 1] Switch btwn Melee and Targeting
  (if (`self.Targeting`)
    (`AbilitySystemComponent.TargetConfirm` (`self.AbilitySystemComp`))
    (else
      (`AbilitySystemComponent.TryActivateAbilityByClass` (`self.AbilitySystemComp`) "/Game/Blueprints/Characters/GameplayAbilities/Melee/GA_Melee.GA_Melee_C" true))))

(event `self.ReceiveBeginPlay`
  ;[1 1 1] BeginPlay
  (`self.AcquireAbilities` (`self.InitialAbilities`)))

(event `self.SwordCollider.OnComponentBeginOverlap`
  (params (OverlappedComponent :type "PrimitiveComponent Object Reference") (OtherActor :type "Actor Object Reference") (OtherComp :type "PrimitiveComponent Object Reference") (OtherBodyIndex :type Integer) (bFromSweep :type Boolean) (SweepResult :type "HitResult Structure (by ref)"))
  ;[1 1 1] Sword Collision Logic
  (if (!= OtherActor self)
    (bind _asbp_character_base (cast `/Game/Blueprints/Characters/BP_CharacterBase` OtherActor))
    (bind _returnvalue (`self.IsOtherHostile` _asbp_character_base self))
    (if _returnvalue
      (`AbilitySystemBlueprintLibrary.SendGameplayEventToActor` self (struct :`TagName` "skill.melee.dealDamage") (make `GameplayEventData` (struct) null OtherActor)))))

(event `self.BP_Die`
  ;[1 1 1] Death
  (bind _returnvalue (`self.PlayAnimMontage` "/Game/Blueprints/Characters/Animation/AM_Death_Shinbi.AM_Death_Shinbi"))
  (`KismetSystemLibrary.Delay` _returnvalue)
  (`self.K2_DestroyActor`))

(event `self.CapsuleComponent.OnComponentBeginOverlap`
  (params (OverlappedComponent :type "PrimitiveComponent Object Reference") (OtherActor :type "Actor Object Reference") (OtherComp :type "PrimitiveComponent Object Reference") (OtherBodyIndex :type Integer) (bFromSweep :type Boolean) (SweepResult :type "HitResult Structure (by ref)"))
  ;[1 1 1] Only Hit enemies once during Dash
  (bind _asbp_character_base (cast `/Game/Blueprints/Characters/BP_CharacterBase` OtherActor))
  (bind _returnvalue (`self.IsOtherHostile` _asbp_character_base self))
  (if _returnvalue
    (if (not (`KismetArrayLibrary.Array_Contains` (`self.OverlapExclude`) _asbp_character_base))
      (`KismetArrayLibrary.Array_AddUnique` (`self.OverlapExclude`) _asbp_character_base)
      (`AbilitySystemBlueprintLibrary.SendGameplayEventToActor` self (struct :`TagName` "skill.dash.dealDamage") (make `GameplayEventData` (struct) null OtherActor)))))

(event `PushCharacter`
  (params (ImpulseDirection :type "Vector Structure") (ImpulseStrength :type "Float (double-precision)") (StunDuration :type "Float (double-precision)"))
  (bind _charactermovement (`self.CharacterMovement`))
  ;[1 1 1] Push Character
  (set `self.OriginalDefaultFriction` (`CharacterMovementComponent.GroundFriction` _charactermovement))
  (set `CharacterMovementComponent.GroundFriction` 0.0 _charactermovement)
  (`CharacterMovementComponent.AddImpulse` (`self.CharacterMovement`) (* ImpulseDirection ImpulseStrength) true)
  (if (> StunDuration 0.0)
    (`self.HitStun` StunDuration))
  (`KismetSystemLibrary.Delay` 0.3)
  (set `CharacterMovementComponent.GroundFriction` (`self.OriginalDefaultFriction`) (`self.CharacterMovement`)))

(event `ToggleCameraControlRotation`
  (params (shouldControlRotation :type Boolean))
  (if shouldControlRotation
    (set `self.bUseControllerRotationYaw` true)
    (set `CharacterMovementComponent.bOrientRotationToMovement` false (`self.CharacterMovement`))
    (else
      (set `self.bUseControllerRotationYaw` false)
      (set `CharacterMovementComponent.bOrientRotationToMovement` true (`self.CharacterMovement`)))))

(fn `SetCollisionToPawn`
  (params (`New Response` :type "ECollisionResponse Enum" :default "ECR_Ignore"))
  (`PrimitiveComponent.SetCollisionResponseToChannel` (`self.CapsuleComponent`) "ECC_Pawn" `New Response`))

(fn `UserConstructionScript`)